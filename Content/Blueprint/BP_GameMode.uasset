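; Game mode for a UI-driven question game that escalates distraction "noise" as the player drags, and switches between menu, main and win screens.
; Drag starts accumulate clicks that advance phases through thresholds, restarting a looping timer that spawns idea widgets with a train horn at random screen positions.
; A click countdown, re-randomized from per-phase ranges, also spawns an enlarged widget at the cursor.
; An all-answers-correct win check exists but is unwired.
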(event `self.ReceiveBeginPlay`
  (set `self.clickBeforeSpawn` 5)
  (`GameplayStatics.PlaySound2D` "/Game/Sound/Classroom_Noise.Classroom_Noise" 3.0 1.0 0.0 null null))

(event `self.ReceiveTick`
  (params (DeltaSeconds :type "Float (single-precision)")))

(event `SetClickBeforeSpawn`
  (set `self.clickBeforeSpawn` (`KismetMathLibrary.RandomIntegerInRange` (`|GetArrayItem` (`self.minForSpawnOnGrab`) (`self.currentPhase`)) (`|GetArrayItem` (`self.maxForSpawnOnGrab`) (`self.currentPhase`)))))

(event `OnDragStart`
  (`/Engine/EditorBlueprintResources/StandardMacros.IncrementInt` (`self.clickStack`)
    (:`  `
      (`self.CheckPhase`))))

(event `CheckPhase`
  (if (>= (`self.currentPhase`) (`KismetArrayLibrary.Array_Length` (`self.phaseStack`)))
    _
    (elif (> (`self.clickStack`) (`|GetArrayItem` (`self.phaseStack`) (`self.currentPhase`)))
      (bind _result (`/Engine/EditorBlueprintResources/StandardMacros.IncrementInt` (`self.currentPhase`))
        (:`  `
          (`KismetSystemLibrary.PrintString` (`KismetStringLibrary.Conv_IntToString` _result))
          (`KismetSystemLibrary.K2_ClearAndInvalidateTimerHandle` (`self.spawnNoiseAtRandomTimerRef`))
          (bind _returnvalue (`KismetSystemLibrary.K2_SetTimer` null "SpawnNoiseOnRandomLocation" (`|GetArrayItem` (`self.timeForRandomSpawn`) (`self.currentPhase`)) true))
          (set `self.spawnNoiseAtRandomTimerRef` _returnvalue)
          (`self.StackUp`))))))

(event `DashingUI`
  (params (DashingUI :type "/Game/Widget/WBP_Idea1 Object Reference") (WidgetLocation :type "Vector2D Structure") (`Dash Direction` :type "Vector2D Structure"))
  (bind (_x _y) (`KismetMathLibrary.BreakVector2D` WidgetLocation))
  (bind (_x_2 _y_2) (`KismetMathLibrary.BreakVector2D` WidgetLocation))
  (bind (_x_3 _y_3) (`KismetMathLibrary.BreakVector2D` `Dash Direction`))
  (bind (_direction _dash) (`Timeline|Dashing UI` :`NewTime` 0.1 :!via `PlayFromStart`)
    (:`Update`
      (`/Engine/EditorBlueprintResources/StandardMacros.IsValid` DashingUI
        (:`Is Valid`
          (bind (_returnvalue_x _returnvalue_y) (`KismetMathLibrary.BreakVector` (`KismetMathLibrary.VLerp` (`KismetMathLibrary.MakeVector` _x_2 _y_2) (`KismetMathLibrary.MakeVector` (+ _x _x_3) (+ _y _y_3)) _dash)))
          (`CanvasPanelSlot.SetPosition` (`WidgetLayoutLibrary.SlotAsCanvasSlot` DashingUI) (`KismetMathLibrary.MakeVector2D` _returnvalue_x _returnvalue_y)))))))

(event `StartGame`
  (`Widget.SetVisibility` (`self.mainMenuRef`) "Hidden")
  (`Widget.SetVisibility` (`self.mainScreenRef`) "Visible"))

(event `OnWin`
  (`Widget.SetVisibility` (`self.mainScreenRef`) "Hidden")
  (`Widget.SetVisibility` (`self.winScreenRef`) "Visible"))

(fn `RandomPositionUpdate`)

(fn `SpawnNoiseOnMouse`
  (returns (NewParam :type Boolean))
  (bind _output_get (set `self.clickBeforeSpawn` (- (`self.clickBeforeSpawn`) 1)))
  (if (<= _output_get 0)
    (bind _returnvalue (`WidgetLayoutLibrary.GetMousePositionOnViewport`))
    (bind _returnvalue_2 (`|CreateWidget` "/Game/Widget/WBP_Idea1.WBP_Idea1_C" (`GameplayStatics.GetPlayerController` 0) "NewEnumerator2"))
    (`Widget.SetRenderScale` _returnvalue_2 (2.3 2.3))
    (`UserWidget.AddToViewport` _returnvalue_2 0)
    (bind (_x _y) (`KismetMathLibrary.BreakVector2D` _returnvalue))
    (`UserWidget.SetPositionInViewport` _returnvalue_2 (`KismetMathLibrary.MakeVector2D` (- _x 50.0) (- _y 50.0)) false)
    (`self.SetClickBeforeSpawn`)
    (`GameplayStatics.PlaySound2D` "/Game/Sound/Train_Horn.Train_Horn" 1.0 1.0 0.0 null null)
    (return false)
    (else
      (return true))))

(fn `SpawnNoiseOnRandomLocation`
  (bind (_x _y) (`KismetMathLibrary.BreakVector2D` (`WidgetLayoutLibrary.GetViewportSize`)))
  (bind _returnvalue (`|CreateWidget` "/Game/Widget/WBP_Idea1.WBP_Idea1_C" (`GameplayStatics.GetPlayerController` 0) "NewEnumerator2"))
  (`UserWidget.AddToViewport` _returnvalue 0)
  (`UserWidget.SetPositionInViewport` _returnvalue (`KismetMathLibrary.MakeVector2D` (`KismetMathLibrary.RandomFloatInRange` 0.0 _x) (`KismetMathLibrary.RandomFloatInRange` 0.0 _y)) false)
  (`GameplayStatics.PlaySound2D` "/Game/Sound/Train_Horn.Train_Horn" 1.0 1.0 0.0 null null))

(fn `UserConstructionScript`)